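; BaseMode is a game mode that sets up local multiplayer when play begins.
; It hides the first controller's mouse cursor and reads the player count from the options string, using an empty option key.
; It creates the additional local players in a loop, then casts each player's pawn to BaseCharacter and sets its PlayerId to the player index.
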(event `self.ReceiveBeginPlay`
  (bind _numplayer (`self.numPlayer`))
  (set `PlayerController.bShowMouseCursor` false (`GameplayStatics.GetPlayerController` 0))
  (set `self.numPlayer` (`KismetStringLibrary.Conv_StringToInt` (`GameplayStatics.ParseOption` (`self.OptionsString`))))
  (for _index (range 1 (+ _numplayer 1))
    (`GameplayStatics.CreatePlayer` _index))
  (for _index_2 (range (+ _numplayer 1))
    (bind _asbase_character (cast `/Game/MultiplayerBP/Blueprints/BaseCharacter` (`GameplayStatics.GetPlayerPawn` _index_2)))
    (set `/Game/MultiplayerBP/Blueprints/BaseCharacter.PlayerId` _index_2 _asbase_character)))

(fn `UserConstructionScript`)