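; Player controller for a multiplayer prop-hunt mode, handling team choice, pawn spawning and player UI.
; Team requests set Hunter or Prop, register the controller with MultiplayerMode and ask it to spawn; death removes it from the prop list.
; SpawnPlayer spawns and possesses the given character, then closes team selection and restores game-only input.
; Client-prefixed events create the selection and timer widgets, with updates forwarding time and messages to the timer.
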(event `self.ReceiveBeginPlay`
  (bind _asmultiplayer_mode (cast `/Game/MultiplayerBP/Blueprints/MultiplayerMode` (`GameplayStatics.GetGameMode`)))
  (set `self.GameMode` _asmultiplayer_mode))

(event `Die`
  (`KismetArrayLibrary.Array_RemoveItem` (`/Game/MultiplayerBP/Blueprints/MultiplayerMode.propPlayers` (`self.GameMode`)) self))

(event `BeHunter`
  (`self.RequestHunter`))

(event `BeProp`
  (`self.RequestProp`))

(event `RequestHunter`
  (set `self.team` 1)
  (`KismetArrayLibrary.Array_Add` (`/Game/MultiplayerBP/Blueprints/MultiplayerMode.hunterPlayers` (`self.GameMode`)) self)
  (`/Game/MultiplayerBP/Blueprints/MultiplayerMode.SpawnHunter` (`self.GameMode`) self))

(event `RequestProp`
  (set `self.team` 2)
  (`KismetArrayLibrary.Array_Add` (`/Game/MultiplayerBP/Blueprints/MultiplayerMode.propPlayers` (`self.GameMode`)) self)
  (`/Game/MultiplayerBP/Blueprints/MultiplayerMode.SpawnProp` (`self.GameMode`) self))

(event `ShowTeamSelection`
  (`self.ClientShowTeamSelection`))

(event `ClientShowTeamSelection`
  (bind _returnvalue (`|CreateWidget` "/Game/MultiplayerBP/Blueprints/TeamSelection.TeamSelection_C"))
  (bind _output_get (set `self.teamSelection` _returnvalue))
  (`UserWidget.AddToViewport` _output_get 0)
  (`WidgetBlueprintLibrary.SetInputMode_GameAndUIEx` self (`self.teamSelection`))
  (set `self.bShowMouseCursor` true))

(event `ShowTimer`
  ;[1 1 1] Timer
  (`self.ClientShowTimer`))

(event `UpdateTimeWidget`
  (params (Time :type Integer))
  (`/Game/MultiplayerBP/Blueprints/TimerWidget.UpdateTimer` (`self.timerWidget`) Time))

(event `ClientShowTimer`
  ;[1 1 1] Timer
  (bind _returnvalue (`|CreateWidget` "/Game/MultiplayerBP/Blueprints/TimerWidget.TimerWidget_C"))
  (bind _output_get (set `self.timerWidget` _returnvalue))
  (`UserWidget.AddToViewport` _output_get 0))

(event `UpdateMessageWidget`
  (params (Message :type String))
  (`/Game/MultiplayerBP/Blueprints/TimerWidget.UpdateMessage` (`self.timerWidget`) Message))

(event `SpawnPlayer`
  (params (Character :type "/Game/MultiplayerBP/Blueprints/BaseCharacter Class Reference") (Transform :type "Transform Structure"))
  (bind _returnvalue (`|SpawnActorFromClass` Character Transform "AdjustIfPossibleButAlwaysSpawn" "OverrideRootScale" null null))
  (`self.Possess` _returnvalue)
  (`self.ClientRemoveTeamSelection`))

(event `ClientRemoveTeamSelection`
  (`Widget.RemoveFromParent` (`self.teamSelection`))
  (`WidgetBlueprintLibrary.SetInputMode_GameOnly` self)
  (set `self.bShowMouseCursor` false))

(fn `UserConstructionScript`)