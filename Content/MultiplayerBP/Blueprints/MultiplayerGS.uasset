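; MultiplayerGS is a multiplayer Game State Blueprint that runs the countdown timer driving phase changes.
; StartTimer sets a looping one-second event that decrements Timer through UpdateTimer.
; When an update finds Timer at zero or below, it pauses the timer and calls NextPhase on MultiplayerMode.
; StopTimer jumps into that same branch, so stopping the countdown also advances the phase.
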(event `UpdateTimer`
  (bind _timer (`self.timer`))
  (if (> _timer 0)
    (`/Engine/EditorBlueprintResources/StandardMacros.DecrementInt` _timer)
    (else
      (`KismetSystemLibrary.K2_PauseTimerHandle` (stale `StartTimer` _returnvalue) :!label _label)
      (bind _asmultiplayer_mode (cast `/Game/MultiplayerBP/Blueprints/MultiplayerMode` (`GameplayStatics.GetGameMode`)))
      (`/Game/MultiplayerBP/Blueprints/MultiplayerMode.NextPhase` _asmultiplayer_mode))))

(event `StartTimer`
  (bind _returnvalue (`KismetSystemLibrary.K2_SetTimerDelegate` (delegate `UpdateTimer`) 1.0 true)))

(event `StopTimer`
  (goto _label))

(fn `UserConstructionScript`)