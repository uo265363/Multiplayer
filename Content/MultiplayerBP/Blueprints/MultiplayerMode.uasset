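; MultiplayerMode is the game mode for a multiplayer hunter-versus-prop match, handling team selection and character spawning.
; On PostLogin it tells each joining MultiplayerControler to show team selection.
; SpawnHunter and SpawnProp events locate a player start by incoming name, a separate one per team.
; Each passes that transform and its team's character class to the controller's SpawnPlayer, which is responsible for the spawn.
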(event `self.K2_PostLogin`
  (params (NewPlayer :type "PlayerController Object Reference"))
  (bind _asmultiplayer_controler (cast `/Game/MultiplayerBP/Blueprints/MultiplayerControler` NewPlayer))
  (`/Game/MultiplayerBP/Blueprints/MultiplayerControler.ShowTeamSelection` _asmultiplayer_controler))

(event `SpawnHunter`
  (params (Controller :type "PlayerController Object Reference"))
  (bind _asmultiplayer_controler (cast `/Game/MultiplayerBP/Blueprints/MultiplayerControler` Controller))
  (`/Game/MultiplayerBP/Blueprints/MultiplayerControler.SpawnPlayer` _asmultiplayer_controler "/Game/MultiplayerBP/Blueprints/HunterCharacter.HunterCharacter_C" (`self.GetTransform` (`self.K2_FindPlayerStart` _asmultiplayer_controler "0"))))

(event `SpawnProp`
  (params (Controller :type "PlayerController Object Reference"))
  (bind _asmultiplayer_controler (cast `/Game/MultiplayerBP/Blueprints/MultiplayerControler` Controller))
  (`/Game/MultiplayerBP/Blueprints/MultiplayerControler.SpawnPlayer` _asmultiplayer_controler "/Game/MultiplayerBP/Blueprints/Props/PropCharacter.PropCharacter_C" (`self.GetTransform` (`self.K2_FindPlayerStart` _asmultiplayer_controler "1"))))

(fn `UserConstructionScript`)