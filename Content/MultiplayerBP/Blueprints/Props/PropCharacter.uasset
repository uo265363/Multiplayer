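; PropCharacter is a multiplayer character that lets the player take control of props in the world.
; Pressing Interact runs a Scan and, when a prop is found, PossessProp disables the character's movement and has the controller possess that prop.
; Die passes the death to MultiplayerControler.
; Both paths get the controller through player index 0 rather than the character's own controller.
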(event `InputAction|Interact`
  (params (Key :type "Key Structure"))
  (:`Pressed`
    (bind (_prop _foundprop) (`self.Scan`))
    (if _foundprop
      (`self.PossessProp` (`GameplayStatics.GetPlayerController` 0) _prop))))

(event `PossessProp`
  (params (Controller :type "PlayerController Object Reference") (Prop :type "/Game/MultiplayerBP/Blueprints/Props/PropCharacter Object Reference"))
  (`CharacterMovementComponent.DisableMovement` (`self.CharacterMovement`))
  (`Controller.Possess` Controller Prop))

(event `Die`
  (bind _asmultiplayer_controler (cast `/Game/MultiplayerBP/Blueprints/MultiplayerControler` (`GameplayStatics.GetPlayerController` 0)))
  (`/Game/MultiplayerBP/Blueprints/MultiplayerControler.Die` _asmultiplayer_controler))

(fn `UserConstructionScript`
  (`parent.UserConstructionScript`))